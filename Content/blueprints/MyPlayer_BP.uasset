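; Player Blueprint that slides its Playerqq component sideways along Y within limits checked against its world position.
; Move Right and Move Left presses enter the negative-Y and positive-Y branches respectively, supplying the key to check.
; Tick re-runs both branches through a Sequence, polling whether those keys are held.
; Each step is a fixed relative offset without sweep or delta-time scaling, so speed depends on frame rate.
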(event `self.ReceiveBeginPlay`)

(event `self.ReceiveTick`
  (params (DeltaSeconds :type "Float (single-precision)"))
  (bind (_returnvalue_x _returnvalue_y) (`KismetMathLibrary.BreakVector` (`SceneComponent.K2_GetComponentLocation` (`self.Playerqq`))))
  (bind (_returnvalue_x_2 _returnvalue_y_2) (`KismetMathLibrary.BreakVector` (`SceneComponent.K2_GetComponentLocation` (`self.Playerqq`))))
  ;[1 1 1] player movement
  (`|ExecutionSequence`
    (:`then_0`
      (if (`PlayerController.IsInputKeyDown` (`GameplayStatics.GetPlayerController` 0) (stale `InputAction|Move Right` Key)) :!label _label
        (if (>= _returnvalue_y_2 -900.0)
          (`SceneComponent.K2_AddRelativeLocation` (`self.Playerqq`) (0.0 -50.0 0.0) false false))))
    (:`then_1`
      (if (`PlayerController.IsInputKeyDown` (`GameplayStatics.GetPlayerController` 0) (stale `InputAction|Move Left` Key)) :!label _label_2
        (if (<= _returnvalue_y 900.0)
          (`SceneComponent.K2_AddRelativeLocation` (`self.Playerqq`) (0.0 50.0 0.0) false false))))))

(event `InputAction|Move Right`
  (params (Key :type "Key Structure"))
  ;[1 1 1] player movement
  (:`Pressed`
    (goto _label)))

(event `InputAction|Move Left`
  (params (Key :type "Key Structure"))
  ;[1 1 1] player movement
  (:`Pressed`
    (goto _label_2)))

(fn `UserConstructionScript`)