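; Player-controlled physics ball that can be bumped once per attempt with an input action that applies a fixed forward-and-up impulse.
; Bumping requires MyGameMode_BP to report the game not over and health remaining.
; Tick resets the ball when it falls too low, or every frame while the game is over, toggling physics to clear motion, calling the game mode's PlayerHealth and re-arming the bump.
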(event `InputAction|Bump the ball`
  (params (Key :type "Key Structure"))
  (:`Pressed`
    (bind _asmy_game_mode_bp (cast `/Game/main/MyGameMode_BP` (`GameplayStatics.GetGameMode`)))
    (if (and (not (`/Game/main/MyGameMode_BP.GameIsOver` _asmy_game_mode_bp)) (> (`/Game/main/MyGameMode_BP.Health` _asmy_game_mode_bp) 0) (`self.CanBumpTheBall`))
      (set `self.CanBumpTheBall` false)
      (`PrimitiveComponent.AddImpulse` (`self.Ball`) (0.0 0.3 0.8) "None" false))))

(event `self.ReceiveBeginPlay`
  (`self.EnableInput` (`GameplayStatics.GetPlayerController` 0)))

(event `self.ReceiveTick`
  (params (DeltaSeconds :type "Float (single-precision)"))
  (bind (_returnvalue_x _returnvalue_y _returnvalue_z) (`KismetMathLibrary.BreakVector` (`SceneComponent.K2_GetComponentLocation` (`self.Ball`))))
  (bind _asmy_game_mode_bp (cast `/Game/main/MyGameMode_BP` (`GameplayStatics.GetGameMode`)))
  (if (or (<= _returnvalue_z -100.0) (`/Game/main/MyGameMode_BP.GameIsOver` _asmy_game_mode_bp))
    (`SceneComponent.K2_SetWorldLocation` (`self.Ball`) (0.0 0.0 40.0) false false)
    (`PrimitiveComponent.SetSimulatePhysics` (`self.Ball`) false)
    (`PrimitiveComponent.SetSimulatePhysics` (`self.Ball`) true)
    (bind _asmy_game_mode_bp_2 (cast `/Game/main/MyGameMode_BP` (`GameplayStatics.GetGameMode`)))
    (`/Game/main/MyGameMode_BP.PlayerHealth` _asmy_game_mode_bp_2)
    (set `self.CanBumpTheBall` true)))

(fn `UserConstructionScript`)