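; Game mode that tracks score and health, ending the game on victory at a score threshold or defeat when health runs out.
; AddScore accumulates points and PlayerHealth removes one health per call, both feeding a shared game-over path.
; That path loads or creates a ScoreSave in a single slot, records the current score, updates the high score and opens the GameOver level.
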(event `self.ReceiveBeginPlay`)

(event `AddScore`
  (params (AddScore :type Integer))
  (bind _score (`self.Score`))
  ;[1 1 1] Victory
  (set `self.Score` (+ AddScore (`self.Score`)))
  (if (>= (`self.Score`) 20)
    ;[1 1 1] Game over and save
    (set `self.GameIsOver` true :!label _label)
    (`GameplayStatics.DoesSaveGameExist` "Slot1")
    (if true
      (bind _returnvalue (`GameplayStatics.LoadGameFromSlot` "Slot1"))
      (bind _asscore_save (cast `/Game/main/ScoreSave` _returnvalue))
      (else
        (`GameplayStatics.CreateSaveGameObject` "/Game/main/ScoreSave.ScoreSave_C")))
    (bind _output_get (set `self.Save` _asscore_save))
    (set `/Game/main/ScoreSave.CurrentScore` _score _output_get)
    (if (> _score (`/Game/main/ScoreSave.HighestScore` _output_get))
      (set `/Game/main/ScoreSave.HighestScore` _score _output_get))
    (`GameplayStatics.SaveGameToSlot` _output_get "Slot1")
    (`GameplayStatics.OpenLevel` "GameOver")))

(event `PlayerHealth`
  ;[1 1 1] Defeat
  (set `self.Health` (- (`self.Health`) 1))
  (if (<= (`self.Health`) 0)
    (goto _label)))

(fn `UserConstructionScript`)